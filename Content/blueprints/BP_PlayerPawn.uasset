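; Player pawn that rolls its static mesh by physics torque and treats any damage as death.
; Forward/backward and left/right axis inputs feed a shared torque call applied as an acceleration change.
; BeginPlay fades the camera in from black.
; The first damage event fades to black, then reloads the current level after a short delay, with DoOnce blocking repeat triggers.
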(event `InputAxis|Move Forward/Backward`
  (params (AxisValue :type "Float (single-precision)"))
  (`PrimitiveComponent.AddTorqueInRadians` (`self.StaticMesh`) (`KismetMathLibrary.MakeVector` AxisValue (stale `InputAxis|Move Left/Right` AxisValue)) "None" true :!label _label))

(event `InputAxis|Move Left/Right`
  (params (AxisValue :type "Float (single-precision)"))
  (goto _label))

(event `self.ReceiveBeginPlay`
  (`PlayerCameraManager.StartCameraFade` (`GameplayStatics.GetPlayerCameraManager` 0) 1.0 0.0 5.0 (struct :`A` 1.0) false true))

(event `self.ReceiveAnyDamage`
  (params (Damage :type "Float (single-precision)") (DamageType :type "DamageType Object Reference") (InstigatedBy :type "Controller Object Reference") (DamageCauser :type "Actor Object Reference"))
  (`/Engine/EditorBlueprintResources/StandardMacros.DoOnce` false
    (:`Completed`
      (`PlayerCameraManager.StartCameraFade` (`GameplayStatics.GetPlayerCameraManager` 0) 0.0 1.0 3.0 (struct :`A` 1.0) false true)
      (`KismetSystemLibrary.Delay` 3.5)
      (bind _returnvalue (`GameplayStatics.GetCurrentLevelName` true))
      (`GameplayStatics.OpenLevel` (`KismetStringLibrary.Conv_StringToName` _returnvalue)))))

(fn `UserConstructionScript`)